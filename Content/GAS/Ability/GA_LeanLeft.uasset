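; Gameplay ability that toggles the Veil character's left lean.
; On a successful commit it stops all leans, then reverses LeanLeft if already leaning left, reverses LeanLeftToRight if leaning right, or otherwise plays LeanLeft.
; Timeline start times are derived from the current LeanAlpha, so each transition continues from the present lean position.
; The lean timelines live on BP_VeilCharacter, and the ability ends immediately after triggering one.
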(event Ability|EventActivateAbility
  (bind _asbp_veil_character (Utilities|Casting|CastToBP_VeilCharacter (Ability|GetAvatarActorfromActorInfo))
    (:then
      (bind _returnvalue (Ability|CommitAbility))
      (if _returnvalue
        (Default|StopAllLeans _asbp_veil_character)
        (if (Variables|/Game/Blueprints/BP_VeilCharacter.BP_VeilCharacter_C|GetLeaningLeft _asbp_veil_character)
          (Components|Timeline|SetNewTime (Variables|/Game/Blueprints/BP_VeilCharacter.BP_VeilCharacter_C|GetLeanLeft _asbp_veil_character) (* (Variables|/Game/Blueprints/BP_VeilCharacter.BP_VeilCharacter_C|GetLeanAlpha _asbp_veil_character) -0.25))
          (Utilities|String|Reverse (Variables|/Game/Blueprints/BP_VeilCharacter.BP_VeilCharacter_C|GetLeanLeft _asbp_veil_character))
          (elif (Variables|/Game/Blueprints/BP_VeilCharacter.BP_VeilCharacter_C|GetLeaningRight _asbp_veil_character)
            (Components|Timeline|SetNewTime (Variables|/Game/Blueprints/BP_VeilCharacter.BP_VeilCharacter_C|GetLeanLeftToRight _asbp_veil_character) (/ (+ (Variables|/Game/Blueprints/BP_VeilCharacter.BP_VeilCharacter_C|GetLeanAlpha _asbp_veil_character) 1.0) 4.0))
            (Utilities|String|Reverse (Variables|/Game/Blueprints/BP_VeilCharacter.BP_VeilCharacter_C|GetLeanLeftToRight _asbp_veil_character))
            (else
              (Components|Timeline|SetNewTime (Variables|/Game/Blueprints/BP_VeilCharacter.BP_VeilCharacter_C|GetLeanLeft _asbp_veil_character) (* (Variables|/Game/Blueprints/BP_VeilCharacter.BP_VeilCharacter_C|GetLeanAlpha _asbp_veil_character) -0.25))
              (Audio|Components|Audio|Play (Variables|/Game/Blueprints/BP_VeilCharacter.BP_VeilCharacter_C|GetLeanLeft _asbp_veil_character)))))
        (Ability|EndAbility)
        (else
          (Ability|EndAbility))))
    (:CastFailed
      (Ability|EndAbility))))

(event Ability|EventOnEndAbility
  (params (bWasCancelled :type Boolean)))