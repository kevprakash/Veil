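; GA_ReleaseTrigger is a gameplay ability that signals a trigger release on the avatar character's currently equipped gun.
; On activation it commits, then casts the avatar to BP_VeilCharacter and its CurrentEquipped item to BP_GunBase.
; The character's ability system applies GE_TriggerRelease to the gun's own ability system component at the ability's level.
; The ability ends immediately, whether it succeeds or any check fails.
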(event Ability|EventActivateAbility
  (bind _returnvalue (Ability|CommitAbility))
  (if _returnvalue
    (bind _asbp_veil_character (Utilities|Casting|CastToBP_VeilCharacter (Ability|GetAvatarActorfromActorInfo))
      (:then
        (bind _asbp_gun_base (Utilities|Casting|CastToBP_GunBase (Variables|/Game/Blueprints/BP_VeilCharacter.BP_VeilCharacter_C|GetCurrentEquipped _asbp_veil_character))
          (:then
            (GameplayEffects|ApplyGameplayEffectToTarget :self (Variables|/Script/Veil.VeilCharacterBase|GetabilitySystemComponent _asbp_veil_character) :GameplayEffectClass "/Game/GAS/Effect/GE_TriggerRelease.GE_TriggerRelease_C" :Target (Variables|/Script/Veil.VeilEquipmentBase|GetabilitySystemComponent _asbp_gun_base) :Level (Math|Conversions|ToFloat(Integer) (Ability|GetAbilityLevel)))
            (Ability|EndAbility))
          (:CastFailed
            (Ability|EndAbility :!label _label))))
      (:CastFailed
        (goto _label)))
    (else
      (goto _label))))

(event Ability|EventOnEndAbility
  (params (bWasCancelled :type Boolean)))