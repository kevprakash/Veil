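; Gameplay ability that lets a Veil character reinforce the destructible wall it is interacting with, spending one of the team's shared reinforcements.
; Activation requires a valid wall without the Health.Reinforced tag and a positive Reinforcements count in the game state.
; Once committed, it toggles the wall's reinforced state, applies GE_Reinforce to the wall's ability system and ends immediately.
; The commit step subtracts the reinforcement from the game state.
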(event Ability|EventActivateAbility
  (bind _asbp_veil_character (Utilities|Casting|CastToBP_VeilCharacter (Ability|GetAvatarActorfromActorInfo))
    (:then
      (bind _returnvalue (Ability|CommitAbility))
      (if _returnvalue
        (Default|ToggleReinforce (.AsDestructible%20Wall (Utilities|Casting|CastToDestructibleWall (Variables|/Game/Blueprints/BP_VeilCharacter.BP_VeilCharacter_C|GetInteractionActor _asbp_veil_character))) true)
        (GameplayEffects|ApplyGameplayEffectToSelf :self (Variables|/Game/MapPieces/DestructibleWall.DestructibleWall_C|GetAbilitySystem (.AsDestructible%20Wall (Utilities|Casting|CastToDestructibleWall (Variables|/Game/Blueprints/BP_VeilCharacter.BP_VeilCharacter_C|GetInteractionActor _asbp_veil_character)))) :GameplayEffectClass "/Game/GAS/Effect/GE_Reinforce.GE_Reinforce_C")
        (Ability|EndAbility)
        (else
          (Ability|EndAbility :!label _label))))
    (:CastFailed
      (goto _label))))

(event Ability|EventOnEndAbility
  (params (bWasCancelled :type Boolean)))

(event Ability|EventCommitExecute
  (Class|VeilGameState|SubtractReinforcement (.AsVeil%20Game%20State (Utilities|Casting|CastToVeilGameState (Game|GetGameState)))))

(fn K2CanActivateAbility
  (params (ActorInfo :type Gameplay%20Ability%20Actor%20Info%20Structure) (Handle :type Gameplay%20Ability%20Spec%20Handle%20Structure))
  (bind _asbp_veil_character (Utilities|Casting|CastToBP_VeilCharacter (.avataractor ActorInfo)))
  (bind _interactionactor (Variables|/Game/Blueprints/BP_VeilCharacter.BP_VeilCharacter_C|GetInteractionActor _asbp_veil_character))
  (bind _asdestructible_wall (Utilities|Casting|CastToDestructibleWall _interactionactor))
  (Utilities|IsValid _asdestructible_wall
    (:Is%20Valid
      (Utilities|HasTag (Variables|/Game/MapPieces/DestructibleWall.DestructibleWall_C|GetAbilitySystem _asdestructible_wall) (GameplayTags|MakeLiteralGameplayTag "(TagName=\"Health.Reinforced\")")
        (:true
          (return "" false))
        (:false
          (return "" (> (Variables|/Script/Veil.VeilGameState|Getreinforcements (.AsVeil%20Game%20State (Utilities|Casting|CastToVeilGameState (Game|GetGameState)))) 0)))))
    (:Is%20Not%20Valid
      (return "" false))))