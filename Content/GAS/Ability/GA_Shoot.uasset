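; GA_Shoot is the Gameplay Ability that fires a single shot from a BP_GunBase avatar.
; It ends immediately if the gun has the Weapon.Cycling tag or the ability fails to commit.
; Otherwise it self-applies GE_Cycle with the gun's cycle time as a SetByCaller magnitude, calls the gun's DealDamage, and adds recoil over that cycle time through the instigator's BP_VeilPlayerController.
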(event Ability|EventActivateAbility
  (bind _asbp_gun_base (Utilities|Casting|CastToBP_GunBase (Ability|GetAvatarActorfromActorInfo))
    (:then
      (Utilities|HasTag (Variables|/Script/Veil.VeilEquipmentBase|GetabilitySystemComponent _asbp_gun_base) (GameplayTags|MakeLiteralGameplayTag "(TagName=\"Weapon.Cycling\")")
        (:true
          (Ability|EndAbility :!label _label))
        (:false
          (bind _returnvalue (Ability|CommitAbility))
          (if _returnvalue
            (bind _returnvalue_2 (Ability|GameplayEffect|AssignTagSetbyCallerMagnitude (GameplayEffects|MakeOutgoingSpec :self (Variables|/Script/Veil.VeilEquipmentBase|GetabilitySystemComponent _asbp_gun_base) :GameplayEffectClass "/Game/GAS/Effect/GE_Cycle.GE_Cycle_C" :Level (Math|Conversions|ToFloat(Integer) (Ability|GetAbilityLevel))) "(TagName=\"Weapon.Cycling\")" (Default|GetCycleTime _asbp_gun_base)))
            (GameplayEffects|ApplyGameplayEffectSpecToSelf (Variables|/Script/Veil.VeilEquipmentBase|GetabilitySystemComponent _asbp_gun_base) _returnvalue_2)
            (Default|DealDamage _asbp_gun_base)
            (Default|AddRecoil (.AsBP%20Veil%20Player%20Controller (Utilities|Casting|CastToBP_VeilPlayerController (Pawn|GetController (Variables|/Script/Engine.Actor|GetInstigator _asbp_gun_base)))) (Default|GetNextRecoil _asbp_gun_base) (Default|GetCycleTime _asbp_gun_base))
            (Ability|EndAbility)
            (else
              (goto _label))))))
    (:CastFailed
      (goto _label))))

(event Ability|EventOnEndAbility
  (params (bWasCancelled :type Boolean)))