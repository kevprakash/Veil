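; GA_PullTrigger is a gameplay ability that fires the gun a BP_VeilCharacter has equipped.
; After committing, it applies GE_TriggerPull from the character's ability system to the gun's own ability system component, at the ability's level.
; It then tries to activate GA_Shoot on the gun, so the shot runs as the weapon's ability.
; The ability ends immediately afterwards, or when a cast or commit fails.
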(event Ability|EventActivateAbility
  (bind _asbp_veil_character (Utilities|Casting|CastToBP_VeilCharacter (Ability|GetAvatarActorfromActorInfo))
    (:then
      (bind _returnvalue (Ability|CommitAbility))
      (if _returnvalue
        (bind _asbp_gun_base (Utilities|Casting|CastToBP_GunBase (Variables|/Game/Blueprints/BP_VeilCharacter.BP_VeilCharacter_C|GetCurrentEquipped _asbp_veil_character))
          (:then
            (GameplayEffects|ApplyGameplayEffectToTarget :self (Variables|/Script/Veil.VeilCharacterBase|GetabilitySystemComponent _asbp_veil_character) :GameplayEffectClass "/Game/GAS/Effect/GE_TriggerPull.GE_TriggerPull_C" :Target (Variables|/Script/Veil.VeilEquipmentBase|GetabilitySystemComponent _asbp_gun_base) :Level (Math|Conversions|ToFloat(Integer) (Ability|GetAbilityLevel)))
            (Abilities|TryActivateAbilitybyClass (Variables|/Script/Veil.VeilEquipmentBase|GetabilitySystemComponent _asbp_gun_base) "/Game/GAS/Ability/GA_Shoot.GA_Shoot_C" true)
            (Ability|EndAbility))
          (:CastFailed
            (Ability|EndAbility :!label _label)))
        (else
          (goto _label))))
    (:CastFailed
      (goto _label))))