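; Player character for Veil, a round-based team shooter with first-person aim, leaning, crouching, interaction, wall reinforcement and bomb planting.
; Authority grants abilities and spawns the primary gun; input drives GAS abilities for firing, reloading, jumping and leaning.
; A crouch timeline feeds server-to-multicast events that adjust capsule, speed and view.
; Damage applies through SetByCaller gameplay effects; zero health triggers death, mesh detachment and spectating.
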(event Custom|UpdateControlRotation
  (bind _returnvalue (Pawn|GetControlRotation :!class /Script/Engine.Pawn))
  (bind _fp_aim (Variables|Default|GetFP%20Aim))
  (bind _returnvalue_2 (Math|Float|Absolute(Float) (.pitch _returnvalue)))
  (bind _returnvalue_3 (< (.pitch _returnvalue) 1.8e+02))
  (bind _returnvalue_4 (- (.pitch _returnvalue) 3.6e+02))
  (bind _returnvalue_5 (Math|Float|Absolute(Float) _returnvalue_4))
  (bind _returnvalue_6 (Math|Float|SelectFloat 1.0 -1.0 _returnvalue_3))
  (bind _returnvalue_7 (Math|Float|Min(Float) _returnvalue_5 _returnvalue_2))
  (bind _returnvalue_8 (* _returnvalue_7 _returnvalue_6))
  (Variables|Default|SetYawPitch (Math|Vector2D|MakeVector2D (.yaw _returnvalue) _returnvalue_8))
  (Transformation|SetRelativeRotation _fp_aim (Math|Rotator|MakeRotator (.roll (Variables|/Script/Engine.SceneComponent|GetRelativeRotation _fp_aim)) _returnvalue_8 0.0) false false))

(event Custom|Equip
  (params (Equipment :type BP%20Veil%20Equipment%20Base%20Object%20Reference))
  (Utilities|IsValid (Variables|Default|GetCurrentEquipped)
    (:Is%20Valid
      (Default|Unequip (Variables|Default|GetCurrentEquipped)))
    (:Is%20Not%20Valid
      _))
  (bind _output_get (Variables|Default|SetCurrentEquipped Equipment))
  (Default|Equip _output_get))

(event Custom|SetCrouchAlphaMulticast
  (params (CrouchAlpha :type Float%20%28double-precision%29))
  (CallFunction|SetCrouchAlpha CrouchAlpha))

(event Custom|Set%20Outline
  (bind _returnvalue (Class|VeilPlayerController|GetTeam (.AsVeil%20Player%20Controller (Utilities|Casting|CastToVeilPlayerController (Game|GetPlayerController 0)))))
  (Rendering|SetCustomDepthStencilValue (Variables|Character|GetMesh) (Math|Integer|SelectInt 1 2 (== (Variables|Default|Getteam) _returnvalue))))

(event Custom|Plant%20Bomb
  (params (SpawnTransform :type Transform))
  (Default|SpawnBomb (.AsBP%20Veil%20Game%20Mode (Utilities|Casting|CastToBP_VeilGameMode (Game|GetGameMode))) SpawnTransform)
  (Class|VeilGameModeBase|SetRoundPhase (.AsVeil%20Game%20Mode%20Base (Utilities|Casting|CastToVeilGameModeBase (Game|GetGameMode))) "POST_PLANT"))

(event Custom|Add%20Damage%20Indicator
  (params (Damage%20Location :type Vector) (Damage :type Float%20%28double-precision%29))
  (bind _returnvalue (UserInterface|CreateWidget "/Game/UI/DamageIndicator.DamageIndicator_C" (Game|GetPlayerController 0)))
  (Variables|/Game/UI/DamageIndicator.DamageIndicator_C|SetDamage%20Location _returnvalue Damage%20Location)
  (Variables|/Game/UI/DamageIndicator.DamageIndicator_C|SetCharacter _returnvalue self)
  (Variables|/Game/UI/DamageIndicator.DamageIndicator_C|SetDuration _returnvalue (Math|Float|Lerp 0.5 2.0 (Math|Float|Clamp(Float) (/ (- Damage 2e+01) 8e+01))))
  (UserInterface|Viewport|AddtoViewport _returnvalue 1))

(event Custom|Activate%20Ability
  (params (InAbilityToActivate :type Gameplay%20Ability%20Class%20Reference))
  (Abilities|TryActivateAbilitybyClass (Variables|Default|GetabilitySystemComponent) InAbilityToActivate true))

(event Custom|Spawn%20Primary
  (params (PrimaryGun :type BP%20Gun%20Base%20Class%20Reference))
  (bind _returnvalue (Game|SpawnActorfromClass PrimaryGun (Transformation|GetActorTransform) "AlwaysSpawn" "MultiplyWithRoot" self 0))
  (bind _output_get (Variables|Default|SetPrimaryGun _returnvalue))
  (Default|BindtoUser _output_get self)
  (CallFunction|Equip _output_get))

(event Custom|On%20Death
  (bind _interactingobject (Variables|Default|GetInteractingObject))
  (if (Utilities|IsValidInterface _interactingobject)
    (Default|CancelInteract _interactingobject self))
  (Utilities|FlowControl|DoOnce false
    (:Completed
      (GameplayEffects|ApplyGameplayEffectToSelf :self (Variables|Default|GetabilitySystemComponent) :GameplayEffectClass "/Game/GAS/Effect/GE_Death.GE_Death_C")
      (Transformation|DetachFromComponent (Variables|Character|GetMesh) "KeepWorld" "KeepWorld" "KeepWorld" true)
      (CallFunction|PostDeathControllerFunctions))))

(event Custom|Set%20FoV
  (params (InFieldOfView :type Float%20%28single-precision%29))
  (Camera|SetFieldOfView (Variables|Default|GetCamera) InFieldOfView))

(event Custom|SetCrouchAlphaServer
  (params (CrouchAlpha :type Float%20%28double-precision%29))
  (CallFunction|SetCrouchAlphaMulticast CrouchAlpha))

(event Custom|SetCrouchAlpha
  (params (CrouchAlpha :type Float%20%28double-precision%29))
  (bind _output_get (Variables|Default|SetCrouchAlpha CrouchAlpha))
  (Components|Capsule|SetCapsuleHalfHeight (Variables|Default|GetCapsuleComponent) (Math|Float|Lerp 1e+02 75.0 _output_get) true)
  (Variables|/Script/Engine.CharacterMovementComponent|SetMaxWalkSpeed (Variables|Character|GetCharacterMovement) (Math|Float|Lerp 4e+02 2.5e+02 _output_get))
  (Transformation|SetRelativeLocation (Variables|Character|GetMesh) (Math|Vector|MakeVector -15.0 -5.0 (- (- 1e+02 (Math|Float|Lerp 1e+02 75.0 _output_get)) 1e+02)) false false)
  (Transformation|SetRelativeLocation (Variables|Default|GetFP%20Aim) (Math|Vector|MakeVector 0.0 0.0 (- 7e+01 (- 1e+02 (Math|Float|Lerp 1e+02 75.0 _output_get)))) false false))

(event Custom|Set%20ADS%20Alpha
  (params (ADSAlpha :type Float%20%28double-precision%29))
  (Variables|Default|SetADSAlpha ADSAlpha))

(event Custom|Reinforce%20Wall
  (params (Wall :type Destructible%20Wall%20Object%20Reference))
  (Variables|Default|SetInteractionActor Wall)
  (Utilities|FlowControl|DelayUntilNextTick)
  (Abilities|TryActivateAbilitybyClass (Variables|Default|GetabilitySystemComponent) "/Game/GAS/Ability/GA_Reinforce.GA_Reinforce_C" true))

(event Input|EnhancedActionEvents|EnhancedInputActionIA_Walk
  (params (ActionValue :type Vector%202D%20Structure) (ElapsedSeconds :type Float%20%28double-precision%29) (TriggeredSeconds :type Float%20%28double-precision%29) (InputAction :type Input%20Action%20Object%20Reference :default "/Game/Input/InputActions/IA_Walk.IA_Walk"))
  (Class|PawnMovementComponent|AddInputVector (Variables|Character|GetCharacterMovement) (Math|Vector|Normalize (Math|Vector|RotateVector (Math|Conversions|ToVector(Vector2D) ActionValue) (Transformation|GetActorRotation))) false))

(event Input|EnhancedActionEvents|EnhancedInputActionIA_AltUse
  (params (ActionValue :type Boolean) (ElapsedSeconds :type Float%20%28double-precision%29) (TriggeredSeconds :type Float%20%28double-precision%29) (InputAction :type Input%20Action%20Object%20Reference :default "/Game/Input/InputActions/IA_AltUse.IA_AltUse"))
  (bind _currentequipped (Variables|Default|GetCurrentEquipped))
  (:Started
    (Utilities|IsValid _currentequipped
      (:Is%20Valid
        (Default|AltUse _currentequipped))))
  (:Completed
    (Utilities|IsValid _currentequipped
      (:Is%20Valid
        (Default|StopAltUse _currentequipped)))))

(event Input|EnhancedActionEvents|EnhancedInputActionIA_Use
  (params (ActionValue :type Boolean) (ElapsedSeconds :type Float%20%28double-precision%29) (TriggeredSeconds :type Float%20%28double-precision%29) (InputAction :type Input%20Action%20Object%20Reference :default "/Game/Input/InputActions/IA_Use.IA_Use"))
  (:Triggered
    (CallFunction|UseCurrentEquipment))
  (:Canceled
    (CallFunction|StopUsingCurrentEquipment :!label _label))
  (:Completed
    (goto _label)))

(event Input|EnhancedActionEvents|EnhancedInputActionIA_Reload
  (params (ActionValue :type Boolean) (ElapsedSeconds :type Float%20%28double-precision%29) (TriggeredSeconds :type Float%20%28double-precision%29) (InputAction :type Input%20Action%20Object%20Reference :default "/Game/Input/InputActions/IA_Reload.IA_Reload"))
  (CallFunction|ActivateAbility "/Game/GAS/Ability/GA_Reload.GA_Reload_C"))

(event Input|EnhancedActionEvents|EnhancedInputActionIA_Crouch
  (params (ActionValue :type Boolean) (ElapsedSeconds :type Float%20%28double-precision%29) (TriggeredSeconds :type Float%20%28double-precision%29) (InputAction :type Input%20Action%20Object%20Reference :default "/Game/Input/InputActions/IA_Crouch.IA_Crouch"))
  (:Triggered
    (bind _alpha (Timeline|CrouchingTimeline Play)
      (:Update
        (CallFunction|SetCrouchAlphaServer _alpha))))
  (:Canceled
    (Timeline|CrouchingTimeline Reverse))
  (:Completed
    (Timeline|CrouchingTimeline Reverse)))

(event Input|EnhancedActionEvents|EnhancedInputActionIA_Jump
  (params (ActionValue :type Boolean) (ElapsedSeconds :type Float%20%28double-precision%29) (TriggeredSeconds :type Float%20%28double-precision%29) (InputAction :type Input%20Action%20Object%20Reference :default "/Game/Input/InputActions/IA_Jump.IA_Jump"))
  (Abilities|TryActivateAbilitybyClass (Variables|Default|GetabilitySystemComponent) "/Game/GAS/Ability/GA_Jump.GA_Jump_C" true)
  (bind _asbp_gun_base (Utilities|Casting|CastToBP_GunBase (Variables|Default|GetCurrentEquipped)))
  (Default|StopAltUse _asbp_gun_base))

(event Input|EnhancedActionEvents|EnhancedInputActionIA_Interact
  (params (ActionValue :type Boolean) (ElapsedSeconds :type Float%20%28double-precision%29) (TriggeredSeconds :type Float%20%28double-precision%29) (InputAction :type Input%20Action%20Object%20Reference :default "/Game/Input/InputActions/IA_Interact.IA_Interact"))
  (:Triggered
    (Utilities|FlowControl|DoOnce false :!label _label
      (:Completed
        (bind _outhits (CallFunction|TracefromCamera 3 2e+02))
        (bind _array_element (Utilities|Array|ForEachLoopwithBreak _outhits :!label _label_2)
          (:LoopBody
            (bind _asinteractable (Utilities|Casting|CastToInteractable (.hitactor _array_element)))
            (bind _can_interact (Default|CanInteract _asinteractable self))
            (Development|PrintString (Utilities|GetDisplayName (.hitactor _array_element)))
            (if _can_interact
              (bind _output_get (Variables|Default|SetInteractingObject _asinteractable))
              (Default|StartInteract _output_get self)
              (goto _label_2 Break)))))))
  (:Completed
    (Utilities|IsValid (Utilities|ToObject(Interface) (Variables|Default|GetInteractingObject))
      (:Is%20Valid
        (Default|CancelInteract (Variables|Default|GetInteractingObject) self)
        (goto _label Reset))
      (:Is%20Not%20Valid
        (goto _label Reset)))))

(event Input|EnhancedActionEvents|EnhancedInputActionIA_LeanRight
  (params (ActionValue :type Boolean) (ElapsedSeconds :type Float%20%28double-precision%29) (TriggeredSeconds :type Float%20%28double-precision%29) (InputAction :type Input%20Action%20Object%20Reference :default "/Game/Input/InputActions/IA_LeanRight.IA_LeanRight"))
  (CallFunction|ActivateAbility "/Game/GAS/Ability/GA_LeanRight.GA_LeanRight_C"))

(event Input|EnhancedActionEvents|EnhancedInputActionIA_LeanLeft
  (params (ActionValue :type Boolean) (ElapsedSeconds :type Float%20%28double-precision%29) (TriggeredSeconds :type Float%20%28double-precision%29) (InputAction :type Input%20Action%20Object%20Reference :default "/Game/Input/InputActions/IA_LeanLeft.IA_LeanLeft"))
  (CallFunction|ActivateAbility "/Game/GAS/Ability/GA_LeanLeft.GA_LeanLeft_C"))

(event EventBeginPlay
  (|CallParentFunction)
  (CallFunction|SetLeanSpeed)
  (Networking|SwitchHasAuthority
    (:Authority
      (CallFunction|GrantNecessaryAbilities)
      (CallFunction|SpawnPrimary "/Game/Blueprints/Equipment/Guns/BP_GunBase.BP_GunBase_C"))))

(event EventOnNoHealth
  (CallFunction|OnDeath))

(event EventTakeDamage
  (params (Dealer :type Ability%20System%20Component%20Object%20Reference) (Amount :type Float%20%28double-precision%29))
  (bind _abilitysystemcomponent (Variables|Default|GetabilitySystemComponent))
  (bind _returnvalue (Ability|GameplayEffect|AssignTagSetbyCallerMagnitude (GameplayEffects|MakeOutgoingSpec :self Dealer :GameplayEffectClass "/Game/GAS/Effect/GE_TakeDamage.GE_TakeDamage_C") "(TagName=\"Health.Damage\")" (* Amount -1.0)))
  (GameplayEffects|ApplyGameplayEffectSpecToTarget Dealer _returnvalue _abilitysystemcomponent)
  (bind _returnvalue_2 (GameplayAttributes|GetAttributeSet _abilitysystemcomponent "/Script/Veil.VeilAttributeSet"))
  (CallFunction|AddDamageIndicator (Transformation|GetActorLocation (Components|GetOwner Dealer)) Amount)
  (Development|PrintString (Utilities|String|ToString(Float) (.currentvalue (Variables|/Script/Veil.VeilAttributeSet|GetHealth (.AsVeil%20Attribute%20Set (Utilities|Casting|CastToVeilAttributeSet _returnvalue_2))))))
  (if (<= (.currentvalue (Variables|/Script/Veil.VeilAttributeSet|GetHealth (.AsVeil%20Attribute%20Set (Utilities|Casting|CastToVeilAttributeSet _returnvalue_2)))) 0.0)
    (Class|Damageable|OnNoHealth(Message) self)))

(fn ConstructionScript)

(fn GrantNecessaryAbilities
  (for _array_element (LocalVariables|GetAbilities)
    (GameplayAbilities|GiveAbility (Variables|Default|GetabilitySystemComponent) _array_element 0 -1)))

(fn UseCurrentEquipment
  (Utilities|Casting|CastToBP_GunBase (Variables|Default|GetCurrentEquipped))
  (CallFunction|ActivateAbility "/Game/GAS/Ability/GA_PullTrigger.GA_PullTrigger_C"))

(fn StopUsingCurrentEquipment
  (Utilities|Casting|CastToBP_GunBase (Variables|Default|GetCurrentEquipped))
  (CallFunction|ActivateAbility "/Game/GAS/Ability/GA_ReleaseTrigger.GA_ReleaseTrigger_C"))

(fn TracefromCamera
  (params (Trace%20Level :type Integer) (Trace%20Length :type Float%20%28single-precision%29) (Spread :type Vector%202D%20Structure))
  (bind _camera (Variables|Default|GetCamera))
  (bind _returnvalue (Transformation|GetWorldLocation _camera))
  (bind _outhits (Collision|MultiLineTraceByChannel _returnvalue (+ _returnvalue (* (Class|KismetMathLibrary|RandomUnitVectorinEllipticalConeinDegrees (Math|Vector|GetForwardVector (Pawn|GetControlRotation :!class /Script/Engine.Pawn)) (.x Spread) (.y Spread)) Trace%20Length)) (Utilities|Select :Index Trace%20Level :Option%200 "TraceTypeQuery5" :Option%201 "TraceTypeQuery4" :Option%202 "TraceTypeQuery3" :Option%203 "TraceTypeQuery6") true (Utilities|Array|MakeArray self) "ForDuration"))
  (return _outhits))

(fn PostDeathControllerFunctions
  (bind _output_get (LocalVariables|SetVeilController (.AsBP%20Veil%20Player%20Controller (Utilities|Casting|CastToBP_VeilPlayerController (Pawn|GetController)))))
  (Pawn|UnPossess _output_get)
  (Default|Spectate _output_get self)
  (Class|VeilGameModeBase|SetPlayerLife (.AsBP%20Veil%20Game%20Mode (Utilities|Casting|CastToBP_VeilGameMode (Game|GetGameMode))) (LocalVariables|GetVeilController) false false))

(fn UpdateLean
  (bind _leanalpha (Variables|Default|GetLeanAlpha))
  (bind _leanmovementdirection (Variables|Default|GetLeanMovementDirection))
  (bind _fp_aim (Variables|Default|GetFP%20Aim))
  (Transformation|SetRelativeLocationAndRotation _fp_aim (Math|Vector|Lerp(Vector) "0.000000,0.000000,70.000000" "0.000000,15.000000,70.000000" _leanalpha) (Math|Rotator|MakeRotator (Math|Float|Lerp 0.0 3e+01 _leanalpha) (.pitch (Variables|/Script/Engine.SceneComponent|GetRelativeRotation _fp_aim)) 0.0) false false)
  (Variables|Default|SetLeaningLeft (and (< _leanalpha 0.0) (not _leanmovementdirection)))
  (Variables|Default|SetLeaningRight (and (> _leanalpha 0.0) _leanmovementdirection)))

(fn SetLeanSpeed
  (bind _lean_speed (LocalVariables|GetLean%20Speed))
  (Components|Timeline|SetPlayRate (Variables|Default|GetLeanLeft) _lean_speed)
  (Components|Timeline|SetPlayRate (Variables|Default|GetLeanRight) _lean_speed)
  (Components|Timeline|SetPlayRate (Variables|Default|GetLeanLeftToRight) _lean_speed))

(fn StopAllLeans
  (Audio|Components|Audio|Stop (Variables|Default|GetLeanLeft))
  (Audio|Components|Audio|Stop (Variables|Default|GetLeanRight))
  (Audio|Components|Audio|Stop (Variables|Default|GetLeanLeftToRight)))