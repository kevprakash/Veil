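; Player controller for Veil that handles look input, round input controls, recoil, view switching and death spectating.
; On possession it grants the Reinforce ability based on team, and round toggles add or remove Enhanced Input mapping contexts.
; Look input and timeline-driven recoil share one yaw/pitch event that updates the character's control rotation.
; On death it possesses a top-down spectator pawn, then after a delay attaches it to the first listed team player.
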(event Custom|Set%20View%20Actor
  (params (Target :type Actor%20Object%20Reference))
  (Game|Player|SetViewTargetwithBlend Target 0.2 "VTBlend_Linear" 0.0 false))

(event Custom|Add%20Recoil
  (params (Amount :type Vector%202D%20Structure) (Duration :type Float%20%28double-precision%29))
  (bind _returnvalue (/ 1.0 Duration))
  (Components|Timeline|SetPlayRate (Variables|Default|GetRecoil) _returnvalue)
  (bind _d (Timeline|Recoil PlayFromStart)
    (:Update
      (CallFunction|AddYawandPitch (.x (* Amount (Utilities|Time|GetWorldDeltaSeconds) _returnvalue _d)) (* (.y (* Amount (Utilities|Time|GetWorldDeltaSeconds) _returnvalue _d)) -1.0)))))

(event Custom|Add%20Yaw%20and%20Pitch
  (params (Yaw :type Float%20%28double-precision%29) (Pitch :type Float%20%28double-precision%29))
  (Class|PlayerController|AddYawInput Yaw)
  (Class|PlayerController|AddPitchInput Pitch)
  (bind _asbp_veil_character (Utilities|Casting|CastToBP_VeilCharacter (Pawn|GetControlledPawn)))
  (Default|UpdateControlRotation _asbp_veil_character))

(event Custom|Spectate
  (params (Death%20Character :type BP%20Veil%20Character%20Object%20Reference))
  (bind _returnvalue (Transformation|GetActorRotation Death%20Character))
  (bind _returnvalue_2 (Game|SpawnActorfromClass "/Game/Blueprints/BP_VeilSpectatorPawn.BP_VeilSpectatorPawn_C" (Math|Transform|MakeTransform (+ (Transformation|GetActorLocation Death%20Character) (* (Transformation|GetActorForwardVector Death%20Character) -1e+02) (* (Transformation|GetActorUpVector Death%20Character) 2e+02)) (Math|Rotator|MakeRotator (.roll _returnvalue) -9e+01 (.yaw _returnvalue)) "1.000000,1.000000,1.000000") "AlwaysSpawn" "MultiplyWithRoot" self 0))
  (Pawn|Possess _returnvalue_2)
  (Utilities|FlowControl|Delay 2.0)
  (bind _view_target (CallFunction|GetSpectateTarget))
  (Utilities|IsValid _view_target
    (:Is%20Valid
      (Default|AttachtoActor _returnvalue_2 _view_target))))

(event Custom|Set%20Round%20Controls
  (params (Add :type Boolean))
  (if Add
    (CallFunction|AddRoundControls)
    (else
      (CallFunction|RemoveRoundControls))))

(event Custom|Add%20Widget%20To%20Viewport
  (params (Class :type User%20Widget%20Class%20Reference))
  (bind _returnvalue (UserInterface|CreateWidget Class self))
  (UserInterface|Viewport|AddtoViewport _returnvalue 0))

(event Input|EnhancedActionEvents|EnhancedInputActionIA_Look
  (params (ActionValue :type Vector%202D%20Structure) (ElapsedSeconds :type Float%20%28double-precision%29) (TriggeredSeconds :type Float%20%28double-precision%29) (InputAction :type Input%20Action%20Object%20Reference :default "/Game/Input/InputActions/IA_Look.IA_Look"))
  (bind _sensitivity (Variables|Default|GetSensitivity))
  (bind _returnvalue (* ActionValue _sensitivity "(X=0.125000,Y=0.125000)"))
  (CallFunction|AddYawandPitch (.x _returnvalue) (* (.y _returnvalue) -1.0)))

(event EventBeginPlay)

(event EventPossess
  (params (PossessedPawn :type Pawn%20Object%20Reference))
  (|CallParentFunction PossessedPawn)
  (bind _asveil_character_base (Utilities|Casting|CastToVeilCharacterBase PossessedPawn))
  (bind _returnvalue (Class|VeilPlayerController|GetTeam))
  (if (Math|Conversions|ToBoolean(Integer) _returnvalue)
    (GameplayAbilities|GiveAbility (Variables|/Script/Veil.VeilCharacterBase|GetabilitySystemComponent _asveil_character_base) "/Game/GAS/Ability/GA_Reinforce.GA_Reinforce_C" 0 -1)
    (else
      (Development|PrintString (Utilities|String|ToString(Integer) _returnvalue)))))

(fn ConstructionScript)

(fn GetSpectateTarget
  (bind _returnvalue (Game|GetGameState))
  (bind _asveil_game_state (Utilities|Casting|CastToVeilGameState _returnvalue))
  (bind _returnvalue_2 (Class|VeilGameState|GetTeam _asveil_game_state self))
  (bind _returnvalue_3 (Class|VeilGameState|GetPlayersonTeam _asveil_game_state _returnvalue_2))
  (bind _array_element (Utilities|Array|ForEachLoopwithBreak _returnvalue_3)
    (:LoopBody
      (return _array_element))
    (:Completed
      (return 0))))

(fn RemoveRoundControls
  (bind _returnvalue (PlayerController|LocalPlayerSubsystems|GetEnhancedInputLocalPlayerSubsystem))
  (Utilities|FlowControl|Sequence
    (:then_0
      (Utilities|IsValid _returnvalue
        (:Is%20Valid
          (Input|RemoveMappingContext _returnvalue "/Game/Input/IMCs/IMC_Equipment.IMC_Equipment" "(bIgnoreAllPressedKeysUntilRelease=True,bForceImmediately=False,bNotifyUserSettings=False)")
          (Input|RemoveMappingContext _returnvalue "/Game/Input/IMCs/IMC_Interaction.IMC_Interaction" "(bIgnoreAllPressedKeysUntilRelease=True,bForceImmediately=False,bNotifyUserSettings=False)"))))
    (:then_1
      (bind _asbp_veil_character (Utilities|Casting|CastToBP_VeilCharacter (Pawn|GetControlledPawn)))
      (Default|StopAltUse (Variables|/Game/Blueprints/BP_VeilCharacter.BP_VeilCharacter_C|GetCurrentEquipped _asbp_veil_character)))))

(fn AddRoundControls
  (bind _returnvalue (PlayerController|LocalPlayerSubsystems|GetEnhancedInputLocalPlayerSubsystem))
  (Utilities|IsValid _returnvalue
    (:Is%20Valid
      (Input|AddMappingContext _returnvalue "/Game/Input/IMCs/IMC_CharacterMovement.IMC_CharacterMovement" 0 "(bIgnoreAllPressedKeysUntilRelease=True,bForceImmediately=False,bNotifyUserSettings=False)")
      (Input|AddMappingContext _returnvalue "/Game/Input/IMCs/IMC_Camera.IMC_Camera" 0 "(bIgnoreAllPressedKeysUntilRelease=True,bForceImmediately=False,bNotifyUserSettings=False)")
      (Input|AddMappingContext _returnvalue "/Game/Input/IMCs/IMC_Equipment.IMC_Equipment" 0 "(bIgnoreAllPressedKeysUntilRelease=True,bForceImmediately=False,bNotifyUserSettings=False)")
      (Input|AddMappingContext _returnvalue "/Game/Input/IMCs/IMC_Interaction.IMC_Interaction" 0 "(bIgnoreAllPressedKeysUntilRelease=True,bForceImmediately=False,bNotifyUserSettings=False)"))))