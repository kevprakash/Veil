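; Destructible wall segment that takes damage through the Gameplay Ability System and can be reset after breaking.
; TakeDamage applies a SetByCaller damage effect from the dealer, updates a dynamic material's Damage parameter from lost health, and sends OnNoHealthMessage at zero health.
; OnNoHealth calls Break on authority, hiding the mesh and disabling collision rather than destroying the actor.
; Reset restores visibility and collision, applies a health-reset effect and refreshes the material.
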(event Custom|Break
  (bind _mesh (Variables|Character|GetMesh))
  (Rendering|SetVisibility _mesh false true)
  (Collision|SetCollisionEnabled _mesh "NoCollision"))

(event Custom|UpdateColour
  (bind _material (Variables|Default|GetMaterial))
  (bind _attributeset (Variables|Default|GetattributeSet))
  (bind _maxhealth (Variables|/Script/Veil.VeilAttributeSet|GetMaxHealth _attributeset))
  (Utilities|IsValid _material
    (:Is%20Valid
      (Rendering|Material|SetScalarParameterValue _material "Damage" (/ (- (.currentvalue _maxhealth) (.currentvalue (Variables|/Script/Veil.VeilAttributeSet|GetHealth _attributeset))) (.currentvalue _maxhealth)) :!class /Script/Engine.MaterialInstanceDynamic))))

(event EventReset
  (bind _mesh (Variables|Character|GetMesh))
  (Rendering|SetVisibility _mesh true true)
  (Collision|SetCollisionEnabled _mesh "QueryAndPhysics")
  (GameplayEffects|ApplyGameplayEffectToSelf :self (Variables|Default|GetabilitySystemComponent) :GameplayEffectClass "/Game/GAS/Effect/GE_ResetHealth.GE_ResetHealth_C")
  (CallFunction|UpdateColour))

(event EventBeginPlay
  (bind _returnvalue (Rendering|Material|CreateDynamicMaterialInstance "/Game/Art/Materials/M_Destructible.M_Destructible" "None" "None" :!class /Script/Engine.KismetMaterialLibrary))
  (bind _output_get (Variables|Default|SetMaterial _returnvalue))
  (Rendering|Material|SetMaterial (Variables|Character|GetMesh) 0 _output_get))

(event EventTick
  (params (DeltaSeconds :type Float%20%28single-precision%29)))

(event EventOnNoHealth
  (Networking|SwitchHasAuthority
    (:Authority
      (CallFunction|Break))))

(event EventTakeDamage
  (params (Dealer :type Ability%20System%20Component%20Object%20Reference) (Amount :type Float%20%28double-precision%29))
  (bind _abilitysystemcomponent (Variables|Default|GetabilitySystemComponent))
  (bind _returnvalue (Ability|GameplayEffect|AssignTagSetbyCallerMagnitude (GameplayEffects|MakeOutgoingSpec :self Dealer :GameplayEffectClass "/Game/GAS/Effect/GE_TakeDamage.GE_TakeDamage_C") "(TagName=\"Health.Damage\")" (* Amount -1.0)))
  (GameplayEffects|ApplyGameplayEffectSpecToTarget Dealer _returnvalue _abilitysystemcomponent)
  (bind _returnvalue_2 (GameplayAttributes|GetAttributeSet _abilitysystemcomponent "/Script/Veil.VeilAttributeSet"))
  (CallFunction|UpdateColour)
  (if (<= (.currentvalue (Variables|/Script/Veil.VeilAttributeSet|GetHealth (.AsVeil%20Attribute%20Set (Utilities|Casting|CastToVeilAttributeSet _returnvalue_2)))) 0.0)
    (Class|Damageable|OnNoHealth(Message) self)))

(fn ConstructionScript)