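; Base Blueprint for equipment used by a Veil character, with separate first-person and third-person meshes.
; BindtoUser stores the user, casts it to BP_VeilCharacter, then snaps Mesh to the first-person gun socket and ThirdPersonMesh to the body's right hand.
; Equip, Unequip and the primary and alternate use start/stop events are empty stubs.
; A node hiding Mesh is left unconnected.
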(event Custom|StopUse)

(event Custom|StopAltUse)

(event Custom|Bind%20to%20User
  (params (User :type BP%20Veil%20Character%20Object%20Reference))
  (bind _output_get (Variables|Default|Setuser User))
  (bind _asbp_veil_character (Utilities|Casting|CastToBP_VeilCharacter _output_get))
  (Transformation|AttachComponentToComponent (Variables|Character|GetMesh) (Variables|/Game/Blueprints/BP_VeilCharacter.BP_VeilCharacter_C|GetFirstPerson%20Mesh _asbp_veil_character) "R_GunSocket" "SnapToTarget" "SnapToTarget" "SnapToTarget" true)
  (Transformation|AttachComponentToComponent (Variables|Default|GetThirdPerson%20Mesh) (Variables|/Script/Engine.Character|GetMesh _asbp_veil_character) "RightHand" "SnapToTarget" "SnapToTarget" "SnapToTarget" true))

(event Custom|Equip)

(event Custom|Unequip)

(event Custom|Use)

(event Custom|AltUse)

(event EventBeginPlay
  (|CallParentFunction))

(fn ConstructionScript)