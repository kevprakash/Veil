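; Base gun equipment built on the Gameplay Ability System, whose attributes drive fire rate, recoil, damage and aiming.
; On authority it grants GA_Shoot and applies attachments as Gameplay Effects, with scope choice also setting sight meshes.
; Alt-use runs a timeline blending FOV and ADS alpha, which tightens spread and toggles ADS effects.
; Damage comes from camera traces with distance falloff, per-actor penetration decay and headshot bonus, keeping each actor's highest hit.
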(event EventBeginPlay
  (|CallParentFunction)
  (Networking|SwitchHasAuthority
    (:Authority
      (CallFunction|GrantNecessaryAbilities)
      (CallFunction|LoadAttachments))))

(event EventUse)

(event EventUnequip
  (Rendering|SetVisibility (Variables|Character|GetMesh) false true))

(event EventEquip
  (Rendering|SetVisibility (Variables|Character|GetMesh) true true))

(event EventAltUse
  (bind _user (Variables|Default|Getuser))
  (bind _user_2 (Variables|Default|Getuser))
  (bind _returnvalue (Ability|GetAbilitySystemComponent _user))
  (bind _asbp_veil_character (Utilities|Casting|CastToBP_VeilCharacter _user_2))
  (bind _adsalpha (Variables|/Game/Blueprints/BP_VeilCharacter.BP_VeilCharacter_C|GetADSAlpha _asbp_veil_character))
  (bind _returnvalue_2 (> _adsalpha 0.8))
  (bind _alpha (Timeline|Zoom Play)
    (:Update
      (Components|Timeline|SetPlayRate (Variables|Default|GetZoom) (/ 1.0 (CallFunction|GetADSTime)))
      (Default|SetFoV _asbp_veil_character (Math|Float|Lerp 104.0 (CallFunction|CalculateFoV) _alpha))
      (Default|SetADSAlpha _asbp_veil_character _alpha)
      (if (!= _returnvalue_2 (GameplayTags|HasMatchingGameplayTag _returnvalue "(TagName=\"Weapon.ADS\")"))
        (GameplayEffects|ApplyGameplayEffectToTarget :self (Variables|Default|GetabilitySystemComponent) :GameplayEffectClass (select _returnvalue_2 "/Game/GAS/Effect/GE_ADS.GE_ADS_C" "/Game/GAS/Effect/GE_UnADS.GE_UnADS_C") :Target _returnvalue)))))

(event EventStopAltUse
  (bind _user (Variables|Default|Getuser))
  (bind _user_2 (Variables|Default|Getuser))
  (bind _returnvalue (Ability|GetAbilitySystemComponent _user))
  (bind _asbp_veil_character (Utilities|Casting|CastToBP_VeilCharacter _user_2))
  (bind _adsalpha (Variables|/Game/Blueprints/BP_VeilCharacter.BP_VeilCharacter_C|GetADSAlpha _asbp_veil_character))
  (bind _returnvalue_2 (> _adsalpha 0.8))
  (bind _alpha (Timeline|Zoom Reverse)
    (:Update
      (Components|Timeline|SetPlayRate (Variables|Default|GetZoom) (/ 1.0 (CallFunction|GetADSTime)))
      (Default|SetFoV _asbp_veil_character (Math|Float|Lerp 104.0 (CallFunction|CalculateFoV) _alpha))
      (Default|SetADSAlpha _asbp_veil_character _alpha)
      (if (!= _returnvalue_2 (GameplayTags|HasMatchingGameplayTag _returnvalue "(TagName=\"Weapon.ADS\")"))
        (GameplayEffects|ApplyGameplayEffectToTarget :self (Variables|Default|GetabilitySystemComponent) :GameplayEffectClass (select _returnvalue_2 "/Game/GAS/Effect/GE_ADS.GE_ADS_C" "/Game/GAS/Effect/GE_UnADS.GE_UnADS_C") :Target _returnvalue)))))

(fn ConstructionScript
  (|CallParentFunction))

(fn GetCycleTime
  (return (/ 6e+01 (.currentvalue (Variables|/Script/Veil.VeilAttributeSet|GetFireRate (Variables|Default|GetattributeSet))))))

(fn GetNextRecoil
  (bind _returnvalue (Math|Random|RandomUnitVectorinConeinDegrees "0.000000,0.000000,1.000000" 9e+01))
  (bind _instabilitycurve (Variables|Default|GetInstabilityCurve))
  (bind _attributeset (Variables|Default|GetattributeSet))
  (bind _attributeset_2 (Variables|Default|GetattributeSet))
  (bind _attributeset_3 (Variables|Default|GetattributeSet))
  (bind _recoilcurve (Variables|Default|GetRecoilCurve))
  (bind _spraycounter (Variables|/Script/Veil.VeilAttributeSet|GetSprayCounter _attributeset))
  (bind _recoilxmultiplier (Variables|/Script/Veil.VeilAttributeSet|GetRecoilXMultiplier _attributeset_3))
  (bind _recoilymultiplier (Variables|/Script/Veil.VeilAttributeSet|GetRecoilYMultiplier _attributeset_3))
  (bind _returnvalue_2 (- (.basevalue _spraycounter) 1.0))
  (bind _returnvalue_3 (Math|Curves|GetVectorValue _instabilitycurve _returnvalue_2))
  (bind _returnvalue_4 (Math|Curves|GetVectorValue _recoilcurve _returnvalue_2))
  (bind _returnvalue_5 (* (.x _returnvalue_4) (.currentvalue _recoilxmultiplier)))
  (bind _returnvalue_6 (* (.y _returnvalue_4) (.currentvalue _recoilymultiplier)))
  (return (Math|Vector2D|MakeVector2D (+ _returnvalue_5 (* _returnvalue_5 (* (* (.x _returnvalue_3) (.currentvalue (Variables|/Script/Veil.VeilAttributeSet|GetInstabilityXMultiplier _attributeset_2))) (.x _returnvalue)))) (+ _returnvalue_6 (* _returnvalue_6 (* (* (.y _returnvalue_3) (.currentvalue (Variables|/Script/Veil.VeilAttributeSet|GetInstabilityYMultiplier _attributeset_2))) (.y _returnvalue)))))))

(fn GrantNecessaryAbilities
  (GameplayAbilities|GiveAbility (Variables|Default|GetabilitySystemComponent) "/Game/GAS/Ability/GA_Shoot.GA_Shoot_C" 0 -1))

(fn DealDamage
  (bind _hit_actors (LocalVariables|GetHit%20Actors))
  (bind _hit_actors_2 (LocalVariables|GetHit%20Actors))
  (bind _hit_actors_3 (LocalVariables|GetHit%20Actors))
  (bind _returnvalue (Utilities|Map|Length _hit_actors_2))
  (bind _outhits (Default|TracefromCamera (.AsBP%20Veil%20Character (Utilities|Casting|CastToBP_VeilCharacter (Variables|Default|Getuser))) 0 1e+04 (CallFunction|CalculateSpread)))
  (for _array_element _outhits
    (if (Utilities|Map|Contains _hit_actors (.hitactor _array_element))
      (if (> (Math|Float|SelectFloat (* (* (CallFunction|GetDamageBaseValue (.distance _array_element)) (Math|Float|Power 0.35 (Math|Conversions|ToFloat(Integer) (Math|Integer|SelectInt (- _returnvalue 1) _returnvalue (Utilities|Map|Contains _hit_actors_2 (.hitactor _array_element)))))) 7.0) (* (CallFunction|GetDamageBaseValue (.distance _array_element)) (Math|Float|Power 0.35 (Math|Conversions|ToFloat(Integer) (Math|Integer|SelectInt (- _returnvalue 1) _returnvalue (Utilities|Map|Contains _hit_actors_2 (.hitactor _array_element)))))) (Components|ComponentHasTag (.hitcomponent _array_element) "Head")) (.Value (Utilities|Map|Find _hit_actors (.hitactor _array_element))))
        (Utilities|Map|Add _hit_actors (.hitactor _array_element) (Math|Float|SelectFloat (* (* (CallFunction|GetDamageBaseValue (.distance _array_element)) (Math|Float|Power 0.35 (Math|Conversions|ToFloat(Integer) (Math|Integer|SelectInt (- _returnvalue 1) _returnvalue (Utilities|Map|Contains _hit_actors_2 (.hitactor _array_element)))))) 7.0) (* (CallFunction|GetDamageBaseValue (.distance _array_element)) (Math|Float|Power 0.35 (Math|Conversions|ToFloat(Integer) (Math|Integer|SelectInt (- _returnvalue 1) _returnvalue (Utilities|Map|Contains _hit_actors_2 (.hitactor _array_element)))))) (Components|ComponentHasTag (.hitcomponent _array_element) "Head"))))
      (else
        (Utilities|Map|Add _hit_actors (.hitactor _array_element) (Math|Float|SelectFloat (* (* (CallFunction|GetDamageBaseValue (.distance _array_element)) (Math|Float|Power 0.35 (Math|Conversions|ToFloat(Integer) (Math|Integer|SelectInt (- _returnvalue 1) _returnvalue (Utilities|Map|Contains _hit_actors_2 (.hitactor _array_element)))))) 7.0) (* (CallFunction|GetDamageBaseValue (.distance _array_element)) (Math|Float|Power 0.35 (Math|Conversions|ToFloat(Integer) (Math|Integer|SelectInt (- _returnvalue 1) _returnvalue (Utilities|Map|Contains _hit_actors_2 (.hitactor _array_element)))))) (Components|ComponentHasTag (.hitcomponent _array_element) "Head"))))))
  (bind _keys (Utilities|Map|Keys _hit_actors_3))
  (for _array_element_2 _keys
    (if (Utilities|DoesObjectImplementInterface _array_element_2 "/Game/Blueprints/Interfaces/Damageable.Damageable_C")
      (Class|Damageable|TakeDamage(Message) _array_element_2 (Variables|Default|GetabilitySystemComponent) (.Value (Utilities|Map|Find _hit_actors_3 _array_element_2))))))

(fn GetDamageBaseValue
  (params (Distance :type Float%20%28double-precision%29))
  (return (* (Math|Curves|GetFloatValue (Variables|Default|GetDamageCurve) (/ Distance 1e+02)) (.currentvalue (Variables|/Script/Veil.VeilAttributeSet|GetDamageMultiplier (Variables|Default|GetattributeSet))))))

(fn CalculateFoV
  (return (* (Class|KismetMathLibrary|DegAtan (/ (Math|Trig|Tan(Degrees) 52.0) (.currentvalue (Variables|/Script/Veil.VeilAttributeSet|GetADSZoom (Variables|Default|GetattributeSet))))) 2.0)))

(fn LoadAttachments
  (params (Params :type Gun%20Data%20Structure))
  (Utilities|FlowControl|Sequence
    (:then_0
      (GameplayEffects|ApplyGameplayEffectToSelf :self (Variables|Default|GetabilitySystemComponent) :GameplayEffectClass (Utilities|Select :Index (.muzzle Params) :NONE "/Game/GAS/Effect/AttachmentEffects/Muzzles/GE_NoBarrel.GE_NoBarrel_C" :FLASH_HIDER "/Game/GAS/Effect/AttachmentEffects/Muzzles/GE_FlashHider.GE_FlashHider_C" :COMPENSATOR "/Game/GAS/Effect/AttachmentEffects/Muzzles/GE_Compensator.GE_Compensator_C" :MUZZLE_BRAKE "/Game/GAS/Effect/AttachmentEffects/Muzzles/GE_MuzzleBreak.GE_MuzzleBreak_C" :EXTENDED_BARREL "/Game/GAS/Effect/AttachmentEffects/Muzzles/GE_ExtendedBarrel.GE_ExtendedBarrel_C" :SUPPRESSOR "/Game/GAS/Effect/AttachmentEffects/Muzzles/GE_Supressor.GE_Supressor_C")))
    (:then_1
      (GameplayEffects|ApplyGameplayEffectToSelf :self (Variables|Default|GetabilitySystemComponent) :GameplayEffectClass (Utilities|Select :Index (.grip Params) :HORIZONTAL "/Game/GAS/Effect/AttachmentEffects/Grips/GE_HorizontalGrip.GE_HorizontalGrip_C" :VERTICAL "/Game/GAS/Effect/AttachmentEffects/Grips/GE_VerticalGrip.GE_VerticalGrip_C" :ANGLED "/Game/GAS/Effect/AttachmentEffects/Grips/GE_AngledGrip.GE_AngledGrip_C" :STUBBY "/Game/GAS/Effect/AttachmentEffects/Grips/GE_StubbyGrip.GE_StubbyGrip_C")))
    (:then_2
      (GameplayEffects|ApplyGameplayEffectToSelf :self (Variables|Default|GetabilitySystemComponent) :GameplayEffectClass (Utilities|Select :Index (.sidebarrel Params) :NONE "/Game/GAS/Effect/AttachmentEffects/SideBarrel/GE_NoSide.GE_NoSide_C" :LASER_SIGHT "/Game/GAS/Effect/AttachmentEffects/SideBarrel/GE_LaserSight.GE_LaserSight_C" :RANGE_FINDER "/Game/GAS/Effect/AttachmentEffects/SideBarrel/GE_RangeFinder.GE_RangeFinder_C")))
    (:then_3
      (GameplayEffects|ApplyGameplayEffectToSelf :self (Variables|Default|GetabilitySystemComponent) :GameplayEffectClass (Utilities|Select :Index (.stock Params) :STANDARD "/Game/GAS/Effect/AttachmentEffects/Stocks/GE_StandardStock.GE_StandardStock_C" :HEAVY_DUTY "/Game/GAS/Effect/AttachmentEffects/Stocks/GE_HeavyDutyStock.GE_HeavyDutyStock_C" :LIGHT "/Game/GAS/Effect/AttachmentEffects/Stocks/GE_LightStock.GE_LightStock_C" :NONE "/Game/GAS/Effect/AttachmentEffects/Stocks/GE_NoStock.GE_NoStock_C")))
    (:then_4
      (GameplayEffects|ApplyGameplayEffectToSelf :self (Variables|Default|GetabilitySystemComponent) :GameplayEffectClass (Utilities|Select :Index (.scope Params) :x1 "/Game/GAS/Effect/AttachmentEffects/Scope/GE_1xScope.GE_1xScope_C" :x2_5 "/Game/GAS/Effect/AttachmentEffects/Scope/GE_2_5xScope.GE_2_5xScope_C" :x4 "/Game/GAS/Effect/AttachmentEffects/Scope/GE_4xScope.GE_4xScope_C" :x8 "/Game/GAS/Effect/AttachmentEffects/Scope/GE_8xScope.GE_8xScope_C"))
      (CallFunction|LoadScope (.scope Params)))))

(fn LoadScope
  (params (Scope :type Scope%20Enum :default "x1"))
  (bind _returnvalue (Utilities|Select :Index Scope :x1 "/Game/FPS_Weapon_Bundle/Weapons/Meshes/Accessories/SM_T4_Sight.SM_T4_Sight" :x2_5 "/Game/FPS_Weapon_Bundle/Weapons/Meshes/Accessories/SM_T4_Sight.SM_T4_Sight" :x4 "/Game/FPS_Weapon_Bundle/Weapons/Meshes/Accessories/SM_Scope_25x56_X.SM_Scope_25x56_X" :x8 "/Game/FPS_Weapon_Bundle/Weapons/Meshes/Accessories/SM_Scope_25x56_X.SM_Scope_25x56_X"))
  (bind _sight (Variables|Default|GetSight))
  (Components|StaticMesh|SetStaticMesh _sight _returnvalue)
  (Components|StaticMesh|SetStaticMesh (Variables|Default|GetThirdPersonSight) _returnvalue)
  (if (Utilities|Array|ContainsItem (Utilities|Array|MakeArray "x4" "x8") Scope)
    (Transformation|SetRelativeLocation _sight "0.000000,15.000000,13.750000" false false)
    (Development|PrintString "Hello")
    (return)
    (else
      (return))))

(fn GetADSTime
  (bind _attributeset (Variables|Default|GetattributeSet))
  (return (/ (.currentvalue (Variables|/Script/Veil.VeilAttributeSet|GetADSTime _attributeset)) (.currentvalue (Variables|/Script/Veil.VeilAttributeSet|GetADSSpeed _attributeset)))))

(fn CalculateSpread
  (bind _user (Variables|Default|Getuser))
  (bind _asbp_veil_character (Utilities|Casting|CastToBP_VeilCharacter _user))
  (bind _adsalpha (Variables|/Game/Blueprints/BP_VeilCharacter.BP_VeilCharacter_C|GetADSAlpha _asbp_veil_character))
  (bind _returnvalue (Math|Float|Lerp 3e+01 0.0 _adsalpha))
  (return (Math|Vector2D|MakeVector2D _returnvalue _returnvalue)))