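; Interactable bomb that players on team 1 can defuse to set the match's win condition.
; Starting an interaction plays the Interaction timeline from the start, and cancelling stops it.
; When the timeline finishes, EndInteract sets the DEFUSED win condition on VeilGameState and destroys the bomb actor.
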(event EventStartInteract
  (params (User :type BP%20Veil%20Character%20Object%20Reference))
  (Timeline|Interaction PlayFromStart
    (:Finished
      (CallFunction|EndInteract User))))

(event EventCancelInteract
  (params (User :type BP%20Veil%20Character%20Object%20Reference))
  (Timeline|Interaction Stop
    (:Finished
      (CallFunction|EndInteract (stale EventStartInteract User)))))

(event EventBeginPlay)

(event EventEndInteract
  (params (User :type BP%20Veil%20Character%20Object%20Reference))
  (Class|VeilGameState|SetWinCondition (.AsVeil%20Game%20State (Utilities|Casting|CastToVeilGameState (Game|GetGameState))) "BOMB_DEFUSED")
  (Actor|DestroyActor))

(fn ConstructionScript)

(fn CanInteract
  (params (User :type BP%20Veil%20Character%20Object%20Reference))
  (bind _returnvalue (Class|VeilCharacterBase|GetTeam User))
  (return (== _returnvalue 1)))