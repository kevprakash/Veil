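; PlantSpot is an interactable bomb plant site that only users on team 0 can use.
; Starting interaction plays the Interaction timeline from the start, cancelling stops it, and completion triggers EndInteract.
; EndInteract calls PlantBomb on the user, passing a spawn transform built from the user's X, Y and rotation and the spot's own Z height.
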(event EventStartInteract
  (params (User :type BP%20Veil%20Character%20Object%20Reference))
  (Timeline|Interaction PlayFromStart
    (:Finished
      (CallFunction|EndInteract User))))

(event EventCancelInteract
  (params (User :type BP%20Veil%20Character%20Object%20Reference))
  (Timeline|Interaction Stop
    (:Finished
      (CallFunction|EndInteract (stale EventStartInteract User)))))

(event EventEndInteract
  (params (User :type BP%20Veil%20Character%20Object%20Reference))
  (bind _returnvalue (Transformation|GetActorLocation User))
  (Default|PlantBomb User (Math|Transform|MakeTransform (Math|Vector|MakeVector (.x _returnvalue) (.y _returnvalue) (.z (Transformation|GetActorLocation))) (Transformation|GetActorRotation User) "1.000000,1.000000,1.000000")))

(fn ConstructionScript)

(fn CanInteract
  (params (User :type BP%20Veil%20Character%20Object%20Reference))
  (bind _returnvalue (Class|VeilCharacterBase|GetTeam User))
  (return (== _returnvalue 0)))