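; Killbox volume actor that kills any BP_VeilCharacter entering its box, such as in a death zone.
; On overlap, only on the server, it builds a GE_TakeDamage spec with a fixed Health.Damage set-by-caller magnitude and applies it to the character's ability system.
; It then calls OnNoHealth directly, regardless of remaining health, and prints the current health value for debugging.
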(event OnComponentBeginOverlap(Box)
  (params (OverlappedComponent :type Primitive%20Component%20Object%20Reference) (OtherActor :type Actor%20Object%20Reference) (OtherComp :type Primitive%20Component%20Object%20Reference) (OtherBodyIndex :type Integer) (bFromSweep :type Boolean) (SweepResult :type Hit%20Result%20Structure%20%28by%20ref%29))
  (Networking|SwitchHasAuthority
    (:Authority
      (bind _asbp_veil_character (Utilities|Casting|CastToBP_VeilCharacter OtherActor))
      (bind _returnvalue (Ability|GameplayEffect|AssignTagSetbyCallerMagnitude (GameplayEffects|MakeOutgoingSpec :self (Variables|/Script/Veil.VeilCharacterBase|GetabilitySystemComponent _asbp_veil_character) :GameplayEffectClass "/Game/GAS/Effect/GE_TakeDamage.GE_TakeDamage_C") "(TagName=\"Health.Damage\")" -2e+02))
      (GameplayEffects|ApplyGameplayEffectSpecToSelf (Variables|/Script/Veil.VeilCharacterBase|GetabilitySystemComponent _asbp_veil_character) _returnvalue)
      (Default|OnNoHealth _asbp_veil_character)
      (Development|PrintString (Utilities|String|ToString(Float) (.currentvalue (Variables|/Script/Veil.VeilAttributeSet|GetHealth (Variables|/Script/Veil.VeilCharacterBase|GetattributeSet _asbp_veil_character))))))))

(event EventBeginPlay)

(event Collision|EventActorBeginOverlap
  (params (OtherActor :type Actor%20Object%20Reference)))

(event EventTick
  (params (DeltaSeconds :type Float%20%28single-precision%29)))

(fn ConstructionScript)